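; BP_Key is a key pickup for a VR door puzzle, with a floating text label that turns to face the player camera every tick.
; A sphere overlap shows the label while a VRPawn is in range.
; TriggerEvent hides the label, disables the sphere and glides the key to a supplied location via a timeline lerp.
; GripEvent glides it to another location, then increments the Door's key count and calls TryOpen.
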(event OnComponentBeginOverlap(Sphere)
  (params (OverlappedComponent :type Primitive%20Component%20Object%20Reference) (OtherActor :type Actor%20Object%20Reference) (OtherComp :type Primitive%20Component%20Object%20Reference) (OtherBodyIndex :type Integer) (bFromSweep :type Boolean) (SweepResult :type Hit%20Result%20Structure%20%28by%20ref%29))
  (Utilities|Casting|CastToVRPawn OtherActor)
  (Rendering|SetVisibility (Variables|Default|GetTextRender) true false))

(event OnComponentEndOverlap(Sphere)
  (params (OverlappedComponent :type Primitive%20Component%20Object%20Reference) (OtherActor :type Actor%20Object%20Reference) (OtherComp :type Primitive%20Component%20Object%20Reference) (OtherBodyIndex :type Integer))
  (Utilities|Casting|CastToVRPawn OtherActor)
  (Rendering|SetVisibility (Variables|Default|GetTextRender) false false))

(event Custom|TriggerEvent
  (params (Location :type Scene%20Component%20Object%20Reference))
  (Variables|Default|SetGoalLocation Location)
  (Rendering|SetVisibility (Variables|Default|GetTextRender) false false)
  (Collision|SetCollisionEnabled (Variables|Default|GetSphere) "NoCollision")
  (bind _alpha (Timeline|Timeline_0 PlayFromStart)
    (:Update
      (Transformation|SetActorLocation (Math|Vector|Lerp(Vector) (Transformation|GetActorLocation) (Transformation|GetWorldLocation (Variables|Default|GetGoalLocation)) _alpha) false false))))

(event Custom|GripEvent
  (params (Location :type Scene%20Component%20Object%20Reference))
  (Variables|Default|SetGoalLocation Location)
  (bind _alpha (Timeline|Timeline_1 PlayFromStart)
    (:Update
      (Transformation|SetActorLocation (Math|Vector|Lerp(Vector) (Transformation|GetActorLocation) (Transformation|GetWorldLocation (Variables|Default|GetGoalLocation)) _alpha) false false))
    (:Finished
      (Utilities|IsValid (Variables|Default|GetDoor)
        (:Is%20Valid
          (Math|Integer|IncrementInt (Variables|/Game/TwoKeys/Blueprints/BP_Door.BP_Door_C|GetCurrentKeyCount (Variables|Default|GetDoor))
            (:%20%20
              (Default|TryOpen (Variables|Default|GetDoor)))))))))

(event EventBeginPlay)

(event Collision|EventActorBeginOverlap
  (params (OtherActor :type Actor%20Object%20Reference)))

(event EventTick
  (params (DeltaSeconds :type Float%20%28single-precision%29))
  (bind _returnvalue (Game|GetPlayerCameraManager 0))
  (bind _textrender (Variables|Default|GetTextRender))
  (bind _returnvalue_2 (Transformation|GetWorldLocation _textrender))
  (bind _returnvalue_3 (Transformation|GetActorLocation _returnvalue))
  (bind _returnvalue_4 (Math|Rotator|FindLookatRotation _returnvalue_2 _returnvalue_3))
  (Transformation|SetWorldRotation _textrender (Math|Rotator|MakeRotator (.roll _returnvalue_4) (.pitch _returnvalue_4) (.yaw _returnvalue_4)) false false))

(fn ConstructionScript)